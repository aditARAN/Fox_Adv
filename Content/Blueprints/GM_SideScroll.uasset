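; GM_SideScroll is a side-scroller game mode Blueprint that tracks the player's lives and gem count and shows them on a HUD widget.
; On BeginPlay it creates the HUD, adds it to the viewport and calls Reset, which restores lives to the maximum and zeroes gems.
; Update_Gems adds a change to the gem total, keeps it from going negative, and pushes the value to the HUD.
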(event Custom|Update_Gems
  (params (Gems :type Integer))
  ;[1 1 1] UPDATE GEMS
  (if (<= (+ Gems (Variables|Default|GetCurr_Gems)) 0)
    (Variables|Default|SetCurr_Gems 0)
    (else
      (Variables|Default|SetCurr_Gems (+ Gems (Variables|Default|GetCurr_Gems)))))
  (Variables|/Game/Blueprints/HUD.HUD_C|SetGems (Variables|Default|GetHUDF) (Variables|Default|GetCurr_Gems)))

(event Custom|Reset
  (bind _max_lives (Variables|Default|GetMax_Lives))
  (bind _hudf (Variables|Default|GetHUDF))
  ;[1 1 1] RESET
  (Variables|Default|SetLives _max_lives)
  (Variables|/Game/Blueprints/HUD.HUD_C|SetLives _hudf _max_lives)
  (Variables|/Game/Blueprints/HUD.HUD_C|SetGems _hudf 0)
  (Variables|Default|SetCurr_Gems 0))

(event EventBeginPlay
  ;[1 1 1] Start
  (bind _returnvalue (UserInterface|CreateWidget "/Game/Blueprints/HUD.HUD_C"))
  (bind _output_get (Variables|Default|SetHUDF _returnvalue))
  (UserInterface|Viewport|AddtoViewport _output_get 0)
  (Class|TypedElementListLibrary|Reset))

(fn ConstructionScript)