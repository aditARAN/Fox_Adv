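; Collectible gem pickup for the side-scroller that adds to the gem tally and then removes itself.
; When BM_SideScroll overlaps its Box, it passes its Gems value to UpdateGems on the GM_SideScroll game mode.
; It then shows the Itemfeedback flipbook for half a second, clears it and destroys the actor.
; Nothing disables the overlap during that delay, so re-entering the Box calls UpdateGems again.
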(event OnComponentBeginOverlap(Box)
  (params (OverlappedComponent :type Primitive%20Component%20Object%20Reference) (OtherActor :type Actor%20Object%20Reference) (OtherComp :type Primitive%20Component%20Object%20Reference) (OtherBodyIndex :type Integer) (bFromSweep :type Boolean) (SweepResult :type Hit%20Result%20Structure%20%28by%20ref%29))
  (Utilities|Casting|CastToBM_SideScroll OtherActor)
  (bind _asgm_side_scroll (Utilities|Casting|CastToGM_SideScroll (Game|GetGameMode)))
  (Default|UpdateGems _asgm_side_scroll (Variables|Default|GetGems))
  (Sprite|SetFlipbook (Variables|Default|GetPaperFlipbook) "/Game/Sunny_Assets/sprites/item-feedback/item-feedback.item-feedback")
  (Utilities|FlowControl|Delay 0.5)
  (Sprite|SetFlipbook (Variables|Default|GetPaperFlipbook))
  (Actor|DestroyActor))

(fn ConstructionScript)